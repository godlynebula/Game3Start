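; BP_EnemyBase is a base enemy character with attack, aggro, walk speed, health and spline patrol logic.
; Attack plays a punch montage and calls AttackFinished on completion or interruption, while aggro swaps the mesh to red and back.
; Point damage drains Health, then ragdolls the mesh with a radial impulse at zero.
; GetPatrolPointLocation steps through PatrolRoute's spline points, reversing at either end.
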(event Custom|Attack
  (Development|PrintText "Attacking!!!")
  (Animation|Montage|PlayMontage (Variables|Character|GetMesh) "/Game/CloseCombatAnimSet/Animations/InPlace/Attacks/NinjaLeftHook_Montage.NinjaLeftHook_Montage"
    (:OnCompleted
      _)
    (:OnInterrupted
      _))
  (Default|CallAttackFinished))

(event Custom|LoseAggro
  (Rendering|Material|SetMaterial (Variables|Character|GetMesh) 0 (Variables|Default|GetOriginalMaterial))
  (Variables|Default|SetbIsAggroed false))

(event Custom|GetAggroed
  (Rendering|Material|SetMaterial (Variables|Character|GetMesh) 0 "/AnimationSharing/AnimSharingRed.AnimSharingRed")
  (Variables|Default|SetbIsAggroed true))

(event Custom|SetWalkSpeed
  (params (Speed :type Float%20%28double-precision%29))
  (Variables|/Script/Engine.CharacterMovementComponent|SetMaxWalkSpeed (Variables|Character|GetCharacterMovement) Speed))

(event Custom|Ragdoll
  (params (Origin :type Vector))
  (Physics|SetSimulatePhysics (Variables|Character|GetMesh) true)
  (Physics|AddRadialImpulse (Variables|Character|GetMesh) (+ Origin "0.000000,0.000000,-100.000000") 3e+02 2.5e+04 "RIF_Constant" false)
  (Pawn|Components|CharacterMovement|DisableMovement (Variables|Character|GetCharacterMovement)))

(event EventBeginPlay
  (Variables|Default|SetOriginalMaterial (Rendering|Material|GetMaterial (Variables|Character|GetMesh) 0)))

(event Game|Damage|EventPointDamage
  (params (Damage :type Float%20%28single-precision%29) (DamageType :type Damage%20Type%20Object%20Reference) (HitLocation :type Vector :default "0, 0, 0") (HitNormal :type Vector :default "0, 0, 0") (HitComponent :type Primitive%20Component%20Object%20Reference) (BoneName :type Name :default "None") (ShotFromDirection :type Vector :default "0, 0, 0") (InstigatedBy :type Controller%20Object%20Reference) (DamageCauser :type Actor%20Object%20Reference) (HitInfo :type Hit%20Result%20Structure%20%28by%20ref%29))
  (Development|PrintText (Utilities|Text|FormatText "{instigator} hit me for {dmg} damage!" InstigatedBy Damage))
  (Variables|Default|SetHealth (- (Variables|Default|GetHealth) Damage))
  (if (<= (Variables|Default|GetHealth) 0.0)
    (Development|PrintText "i ded")
    (CallFunction|Ragdoll ShotFromDirection)))

(fn ConstructionScript)

(fn GetPatrolPointLocation
  (Variables|PatrolRoute|SetPatrolIndex (+ (Variables|PatrolRoute|GetPatrolIndex) (Variables|PatrolRoute|GetDirection))) ; Go to next point
  (if (>= (Variables|PatrolRoute|GetPatrolIndex) (- (Spline|GetNumberOfSplinePoints (Variables|/Game/Blueprints/BP_PatrolRoute.BP_PatrolRoute_C|GetSpline (Variables|PatrolRoute|GetPatrolRoute))) 1))
    (Variables|PatrolRoute|SetDirection -1)
    (elif (<= (Variables|PatrolRoute|GetPatrolIndex) 0)
      (Variables|PatrolRoute|SetDirection 1)))
  (return (Spline|GetLocationatSplinePoint (Variables|/Game/Blueprints/BP_PatrolRoute.BP_PatrolRoute_C|GetSpline (Variables|PatrolRoute|GetPatrolRoute)) (Variables|PatrolRoute|GetPatrolIndex) "World")))