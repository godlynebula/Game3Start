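; BP_ProgPrac is a Blueprint practice actor that spawns random pickups around itself every two seconds.
; On BeginPlay it randomizes HasKey, prints score, health, key and player name, starts spawning and draws a debug circle of the spawn radius.
; SpawnPickUp picks a random class from the ProgPrac array, places it within that horizontal radius using a flattened random unit vector, then re-calls itself after a Delay.
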(event Custom|SpawnPickUp
  (bind _radius (Variables|Default|GetRadius))
  (bind _progprac (Variables|Default|GetProgPrac))
  (Game|SpawnActorfromClass (Utilities|Array|Get(acopy) _progprac (Math|Random|RandomIntegerinRange 0 (- (Utilities|Array|Length _progprac) 1))) (Math|Transform|MakeTransform (+ (Transformation|GetWorldLocation (Variables|Default|GetDefaultSceneRoot)) (* (Math|Random|RandomUnitVector) (Math|Vector|MakeVector _radius _radius 0.0))) "0, 0, 0" "1.000000,1.000000,1.000000") "Undefined" "MultiplyWithRoot" 0 0)
  (Utilities|FlowControl|Delay 2.0)
  (CallFunction|SpawnPickUp))

(event EventBeginPlay
  (Variables|Default|SetHasKey (> (Math|Random|RandomFloat) 0.5))
  (Development|PrintString (Utilities|String|Append (Utilities|String|ToString(Integer) (Variables|Default|GetScore)) (Utilities|String|ToString(Float) (Variables|Default|GetHealth)) (Utilities|String|ToString(Boolean) (Variables|Default|GetHasKey)) (Variables|Default|GetPlayerName)))
  (CallFunction|SpawnPickUp)
  (Rendering|Debug|DrawDebugCircle (Transformation|GetWorldLocation (Variables|Default|GetDefaultSceneRoot)) (Variables|Default|GetRadius) 30 "(R=1.000000,G=0.180736,B=0.000000,A=1.000000)" 6e+01 5.0 "0.000000,1.000000,0.000000" "1.000000,0.000000,0.000000"))

(fn ConstructionScript)