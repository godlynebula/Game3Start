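; BP_Binoculars is a held item that the player can pick up, use to zoom the camera and drop.
; Pickup snaps it to the BPI_ItemSocket on the supplied skeletal mesh and disables Box collision.
; Primary and secondary use each run a FlipFlop setting the third-person character's FollowCamera FOV for normal zoom or extra zoom.
; Drop detaches the Cylinder, enables its physics and collision, and restores its world location.
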(event EventBeginPlay)

(event Collision|EventActorBeginOverlap
  (params (OtherActor :type Actor%20Object%20Reference)))

(event EventTick
  (params (DeltaSeconds :type Float%20%28single-precision%29)))

(event EventPickup
  (params (Skeletal%20Mesh :type Skeletal%20Mesh%20Component%20Object%20Reference))
  (Development|PrintText "These binoculars are being picked up!")
  (Transformation|AttachComponentToComponent Skeletal%20Mesh "BPI_ItemSocket" "SnapToTarget" "SnapToTarget" "KeepRelative" true)
  (Collision|SetCollisionEnabled (Variables|Default|GetBox) "NoCollision"))

(event EventUsePrimary
  (Development|PrintText "Toggle Binocular Zoom On/Off.")
  (Utilities|FlowControl|FlipFlop
    (:A
      (bind _asbp_third_person_character (Utilities|Casting|CastToBP_ThirdPersonCharacter (Game|GetPlayerCharacter 0)))
      (Variables|/Script/Engine.CameraComponent|SetFieldOfView (Variables|/Game/ThirdPerson/Blueprints/BP_ThirdPersonCharacter.BP_ThirdPersonCharacter_C|GetFollowCamera _asbp_third_person_character) 3e+01))
    (:B
      (bind _asbp_third_person_character_2 (Utilities|Casting|CastToBP_ThirdPersonCharacter (Game|GetPlayerCharacter 0)))
      (Variables|/Script/Engine.CameraComponent|SetFieldOfView (Variables|/Game/ThirdPerson/Blueprints/BP_ThirdPersonCharacter.BP_ThirdPersonCharacter_C|GetFollowCamera _asbp_third_person_character_2) 9e+01))))

(event EventUseSecondary
  (Development|PrintText "Zooming in Extra!")
  (Utilities|FlowControl|FlipFlop
    (:A
      (bind _asbp_third_person_character (Utilities|Casting|CastToBP_ThirdPersonCharacter (Game|GetPlayerCharacter 0)))
      (Variables|/Script/Engine.CameraComponent|SetFieldOfView (Variables|/Game/ThirdPerson/Blueprints/BP_ThirdPersonCharacter.BP_ThirdPersonCharacter_C|GetFollowCamera _asbp_third_person_character) 1e+01))
    (:B
      (bind _asbp_third_person_character_2 (Utilities|Casting|CastToBP_ThirdPersonCharacter (Game|GetPlayerCharacter 0)))
      (Variables|/Script/Engine.CameraComponent|SetFieldOfView (Variables|/Game/ThirdPerson/Blueprints/BP_ThirdPersonCharacter.BP_ThirdPersonCharacter_C|GetFollowCamera _asbp_third_person_character_2) 3e+01))))

(event EventDrop
  (bind _cylinder (Variables|Default|GetCylinder))
  (Variables|Default|SetDropLocation (Transformation|GetWorldLocation _cylinder))
  (Transformation|DetachFromComponent _cylinder "KeepRelative" "KeepRelative" "KeepRelative" true) ; Don't follow the hand anymore
  (Physics|SetSimulatePhysics (Variables|Default|GetCylinder) true) ; use gravity to fall
  (Collision|SetCollisionEnabled (Variables|Default|GetCylinder) "QueryAndPhysics") ; Collide with the ground please
  (Transformation|SetWorldLocation (Variables|Default|GetCylinder) (Variables|Default|GetDropLocation) false false) ; To prevent the can from going to world origin
)

(fn ConstructionScript)