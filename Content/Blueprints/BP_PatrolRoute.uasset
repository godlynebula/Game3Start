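; Patrol route Blueprint that hands out successive world-space waypoints from a spline.
; GetPatrolPointLocation steps PatrolIndex by Direction and returns that spline point's location, reversing Direction at either end for back-and-forth movement.
; The upper check triggers only once the index reaches the point count, so that out-of-range index is still queried.
; An unconnected draft of a simpler direction flip remains unused.
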(fn ConstructionScript)

(fn GetPatrolPointLocation
  (Variables|Default|SetPatrolIndex (+ (Variables|Default|GetPatrolIndex) (Variables|Default|GetDirection))) ; Go to next point
  (if (>= (Variables|Default|GetPatrolIndex) (Spline|GetNumberOfSplinePoints (Variables|Default|GetSpline)))
    (Variables|Default|SetDirection -1)
    (elif (<= (Variables|Default|GetPatrolIndex) 0)
      (Variables|Default|SetDirection 1)))
  (return (Spline|GetLocationatSplinePoint (Variables|Default|GetSpline) (Variables|Default|GetPatrolIndex) "World")))