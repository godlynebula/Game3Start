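; BP_SpawnEnemyManager populates the level with randomized AI enemies when play begins.
; On BeginPlay it gathers every BP_EnemySpawnPoint, prints their count, and gives each a weighted chance to spawn a BP_AiMoveTo at its transform, owned by that point.
; Each spawned enemy gets a random name label, skeletal mesh and two material slots picked independently from the manager's arrays.
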(event EventBeginPlay
  (bind _enemymaterials (Variables|Default|GetEnemyMaterials))
  (bind _outitem (Utilities|Array|Random _enemymaterials))
  (bind _outactors (Actor|GetAllActorsOfClass "/Game/Blueprints/BP_EnemySpawnPoint.BP_EnemySpawnPoint_C")) ; Finds all BP_EnemySpawnPoint actors
  (Development|PrintText (Utilities|Text|FormatText "There are {count} spawn points in the level." (Utilities|Array|Length _outactors)))
  (for _array_element _outactors
    (if (Math|Random|RandomBoolwithWeight 0.75)
      (bind _returnvalue (Game|SpawnActorfromClass "/Game/AI_Blueprints/BP_AiMoveTo.BP_AiMoveTo_C" (Transformation|GetActorTransform _array_element) "Undefined" "MultiplyWithRoot" _array_element 0))
      (Rendering|Components|TextRender|SetText (Variables|/Game/AI_Blueprints/BP_AiMoveTo.BP_AiMoveTo_C|GetAI%20Name%20Text _returnvalue) (Utilities|Text|ToText(String) (.OutItem (Utilities|Array|Random (Variables|Default|GetEnemyNames)))))
      (Rendering|Material|SetMaterial (Variables|/Script/Engine.Character|GetMesh _returnvalue) 0 _outitem)
      (Rendering|Material|SetMaterial (Variables|/Script/Engine.Character|GetMesh _returnvalue) 1 _outitem)
      (Components|SkeletalMesh|SetSkeletalMeshAsset (Variables|/Script/Engine.Character|GetMesh _returnvalue) (.OutItem (Utilities|Array|Random (Variables|Default|GetEnemyMeshes)))))))

(event Collision|EventActorBeginOverlap
  (params (OtherActor :type Actor%20Object%20Reference)))

(event EventTick
  (params (DeltaSeconds :type Float%20%28single-precision%29)))

(fn ConstructionScript)