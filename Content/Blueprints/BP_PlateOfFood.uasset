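; BP_PlateOfFood is a holdable food item that can be picked up, dropped, eaten and drunk.
; Pickup attaches it to a socket on the given skeletal mesh and disables box collision.
; Drop detaches the cube and restores physics and collision at its current location.
; Primary use eats and secondary use drinks, each once, guarded by booleans that accompany hiding the consumed meshes and printing status text.
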(event EventBeginPlay)

(event Collision|EventActorBeginOverlap
  (params (OtherActor :type Actor%20Object%20Reference)))

(event EventTick
  (params (DeltaSeconds :type Float%20%28single-precision%29)))

(event EventPickup
  (params (Skeletal%20Mesh :type Skeletal%20Mesh%20Component%20Object%20Reference))
  (Development|PrintText "This food is being picked up!")
  (Transformation|AttachComponentToComponent Skeletal%20Mesh "BPI_ItemSocket" "SnapToTarget" "SnapToTarget" "KeepRelative" true)
  (Collision|SetCollisionEnabled (Variables|Default|GetBox) "NoCollision"))

(event EventUsePrimary
  (if (Variables|Default|GetbIsEaten)
    (Development|PrintText "You've already eaten the food!")
    (else
      (Development|PrintText "You ate the food!")
      (Variables|Default|SetbIsEaten true)
      (Rendering|SetVisibility (Variables|Default|GetCube1) false false))))

(event EventDrop
  (bind _cube (Variables|Default|GetCube))
  (Variables|Default|SetDropLocation (Transformation|GetWorldLocation _cube))
  (Transformation|DetachFromComponent _cube "KeepRelative" "KeepRelative" "KeepRelative" true)
  (Physics|SetSimulatePhysics (Variables|Default|GetCube) true)
  (Collision|SetCollisionEnabled (Variables|Default|GetCube) "QueryAndPhysics")
  (Transformation|SetWorldLocation (Variables|Default|GetCube) (Variables|Default|GetDropLocation) false false))

(event EventUseSecondary
  (if (Variables|Default|GetbIsDrinked)
    (Development|PrintText "You have already drinked the beverage!")
    (else
      (Development|PrintText "You drank the beverage!")
      (Variables|Default|SetbIsDrinked true)
      (Rendering|SetVisibility (Variables|Default|GetCylinder) false false))))

(fn ConstructionScript)