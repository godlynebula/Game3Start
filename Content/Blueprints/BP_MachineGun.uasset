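; BP_MachineGun is a machine gun item actor that can be picked up, used and dropped.
; Pickup attaches it to the given skeletal mesh's BPI_ItemSocket and disables body collision.
; UsePrimary is a placeholder that only prints firing text.
; Drop detaches the gun and simulates physics on its body for a short delay, leaving collision disabled throughout.
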(event EventBeginPlay)

(event Collision|EventActorBeginOverlap
  (params (OtherActor :type Actor%20Object%20Reference)))

(event EventTick
  (params (DeltaSeconds :type Float%20%28single-precision%29)))

(event EventPickup
  (params (Skeletal%20Mesh :type Skeletal%20Mesh%20Component%20Object%20Reference))
  (Development|PrintText (Utilities|Text|FormatText "{name} is getting picked up and attached to {mesh}" (Utilities|Text|MakeLiteralText "Machine Gun") Skeletal%20Mesh))
  (Transformation|AttachComponentToComponent Skeletal%20Mesh "BPI_ItemSocket" "SnapToTarget" "SnapToTarget" "KeepRelative" true)
  (Collision|SetCollisionEnabled (Variables|Default|GetMachineGunBody) "NoCollision"))

(event EventUsePrimary
  (Development|PrintText "Pew Pew Pew..."))

(event EventDrop
  (Transformation|DetachFromActor "KeepWorld" "KeepWorld" "KeepRelative")
  (Physics|SetSimulatePhysics (Variables|Default|GetMachineGunBody) true)
  (Collision|SetCollisionEnabled (Variables|Default|GetMachineGunBody) "NoCollision")
  (Utilities|FlowControl|Delay 2.0)
  (Physics|SetSimulatePhysics (Variables|Default|GetMachineGunBody) false))

(fn ConstructionScript)