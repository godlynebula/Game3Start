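; GameMode that saves and loads player stats and per-level world state through SaveGame objects.
; On BeginPlay it restores Health, Mana and Stamina to the third-person character from "PlayerSave", and loads level state from a slot named after the level, creating either save object if missing.
; Level loading replays collected coins and opened doors, with the door loop nested inside the coin loop.
; Separate save events write the held objects to their slots.
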(event Custom|Load%20Player%20Stats
  ;[0.15 0.15 0.15 0.5] Load Player Stats and Save Player Stats Mechanics
  (bind _returnvalue (SaveGame|DoesSaveGameExist "PlayerSave"))
  (if _returnvalue
    (bind _returnvalue_2 (SaveGame|LoadGamefromSlot "PlayerSave"))
    (bind _assg_player_stats (Utilities|Casting|CastToSG_PlayerStats _returnvalue_2))
    (Variables|Default|SetSG_PlayerStats _assg_player_stats)
    (bind _asbp_third_person_character (Utilities|Casting|CastToBP_ThirdPersonCharacter (Game|GetPlayerCharacter 0)))
    (Variables|/Game/ThirdPerson/Blueprints/BP_ThirdPersonCharacter.BP_ThirdPersonCharacter_C|SetStamina _asbp_third_person_character (Variables|/Game/Blueprints/SavingLoading/SG_PlayerStats.SG_PlayerStats_C|GetStamina (Variables|Default|GetSG_PlayerStats)))
    (Variables|/Game/ThirdPerson/Blueprints/BP_ThirdPersonCharacter.BP_ThirdPersonCharacter_C|SetHealth _asbp_third_person_character (Variables|/Game/Blueprints/SavingLoading/SG_PlayerStats.SG_PlayerStats_C|GetHealth (Variables|Default|GetSG_PlayerStats)))
    (Variables|/Game/ThirdPerson/Blueprints/BP_ThirdPersonCharacter.BP_ThirdPersonCharacter_C|SetMana _asbp_third_person_character (Variables|/Game/Blueprints/SavingLoading/SG_PlayerStats.SG_PlayerStats_C|GetMana (Variables|Default|GetSG_PlayerStats)))
    (Development|PrintString "PlayerStats have been loaded." true true "(R=1.000000,G=0.936946,B=0.340872,A=1.000000)" 8.0)
    (else
      (bind _returnvalue_3 (SaveGame|CreateSaveGameObject "/Game/Blueprints/SavingLoading/SG_PlayerStats.SG_PlayerStats_C"))
      (Variables|Default|SetSG_PlayerStats _returnvalue_3))))

(event Custom|Save%20Player%20Stats
  ;[0.15 0.15 0.15 0.5] Load Player Stats and Save Player Stats Mechanics
  (bind _returnvalue (SaveGame|SaveGametoSlot (Variables|Default|GetSG_PlayerStats) "PlayerSave"))
  (if _returnvalue
    (Development|PrintText "PlayerStats written to file." true true "(R=0.270279,G=1.000000,B=0.473983,A=1.000000)")
    (else
      (Development|PrintText "PlayerStats could not be written to file." true true "(R=0.270279,G=1.000000,B=0.473983,A=1.000000)"))))

(event Custom|SaveLevelStateToFile
  ;[0.15 0.15 0.15 0.5] Load Level State and Save Level State Mechanics
  (bind _returnvalue (Game|GetCurrentLevelName true))
  (SaveGame|SaveGametoSlot (Variables|Default|GetSG_LevelState) _returnvalue)
  (if true
    (Development|PrintText "Level State Saved" true true "(R=0.270279,G=1.000000,B=0.473982,A=1.000000)")
    (else
      (Development|PrintText "Save Failed" true true "(R=1.000000,G=0.347200,B=0.558946,A=1.000000)"))))

(event Custom|LoadLevelStateFromFile
  ;[0.15 0.15 0.15 0.5] Load Level State and Save Level State Mechanics
  (bind _returnvalue (Game|GetCurrentLevelName true))
  (bind _returnvalue_2 (SaveGame|DoesSaveGameExist _returnvalue))
  (if _returnvalue_2
    (bind _returnvalue_3 (SaveGame|LoadGamefromSlot _returnvalue))
    (bind _assg_level_state (Utilities|Casting|CastToSG_LevelState _returnvalue_3))
    (Variables|Default|SetSG_LevelState _assg_level_state)
    (for _array_element (Variables|/Game/Blueprints/SavingLoading/SG_LevelState.SG_LevelState_C|GetCollectedCoins (Variables|Default|GetSG_LevelState))
      (Utilities|IsValid _array_element
        (:Is%20Valid
          (Default|CollectThyself _array_element)
          (for _array_element_2 (Variables|/Game/Blueprints/SavingLoading/SG_LevelState.SG_LevelState_C|GetOpenedDoors (Variables|Default|GetSG_LevelState))
            (Utilities|IsValid _array_element_2
              (:Is%20Valid
                (Default|OpenThyself _array_element_2)))))))
    (else
      (bind _returnvalue_4 (SaveGame|CreateSaveGameObject "/Game/Blueprints/SavingLoading/SG_LevelState.SG_LevelState_C"))
      (Variables|Default|SetSG_LevelState _returnvalue_4))))

(event EventBeginPlay
  ;[0.15 0.15 0.15 0.5] On Begin Play, Load Player Stats and Level State
  (Development|PrintString "Loading the SaveLoad GameMode" true true "(R=1.000000,G=0.757305,B=0.286190,A=1.000000)" 1e+01)
  (CallFunction|LoadPlayerStats)
  (CallFunction|LoadLevelStatefromFile))

(fn ConstructionScript)