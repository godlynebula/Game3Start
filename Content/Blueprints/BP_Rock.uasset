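; BP_Rock is a rock item that can be picked up, dropped and thrown.
; Pickup attaches it to a skeletal mesh socket and disables its Box collision, while Drop detaches it with physics and collision at its current location.
; UsePrimary detaches it and launches it through ProjectileMovement using the camera's forward vector.
; UseSecondary is empty, and the impulse throw using ThrowStrength is left unconnected.
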(event EventBeginPlay)

(event Collision|EventActorBeginOverlap
  (params (OtherActor :type Actor%20Object%20Reference)))

(event EventTick
  (params (DeltaSeconds :type Float%20%28single-precision%29)))

(event EventUsePrimary
  (Transformation|DetachFromComponent (Variables|Default|GetRock) "KeepRelative" "KeepRelative" "KeepRelative" true)
  (Collision|SetCollisionEnabled (Variables|Default|GetRock) "QueryAndPhysics") ; Collide with the ground please
  (Components|Activation|Activate (Variables|Default|GetProjectileMovement) false)
  (Game|Components|ProjectileMovement|SetVelocityinLocalSpace (Variables|Default|GetProjectileMovement) (Math|Vector|GetForwardVector (Camera|GetCameraRotation (Variables|/Script/Engine.PlayerController|GetPlayerCameraManager (Game|GetPlayerController 0))))))

(event EventUseSecondary)

(event EventPickup
  (params (Skeletal%20Mesh :type Skeletal%20Mesh%20Component%20Object%20Reference))
  (Development|PrintText "These binoculars are being picked up!")
  (Transformation|AttachComponentToComponent Skeletal%20Mesh "BPI_ItemSocket" "SnapToTarget" "SnapToTarget" "KeepRelative" true)
  (Collision|SetCollisionEnabled (Variables|Default|GetBox) "NoCollision"))

(event EventDrop
  (bind _rock (Variables|Default|GetRock))
  (Variables|Default|SetDropLocation (Transformation|GetWorldLocation _rock))
  (Transformation|DetachFromComponent _rock "KeepRelative" "KeepRelative" "KeepRelative" true) ; Don't follow the hand anymore
  (Physics|SetSimulatePhysics (Variables|Default|GetRock) true) ; use gravity to fall
  (Collision|SetCollisionEnabled (Variables|Default|GetRock) "QueryAndPhysics") ; Collide with the ground please
  (Transformation|SetWorldLocation (Variables|Default|GetRock) (Variables|Default|GetDropLocation) false false) ; To prevent the can from going to world origin
)

(fn ConstructionScript)