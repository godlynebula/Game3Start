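; Demo Blueprint for loop and list flow control, reporting its progress through on-screen debug prints.
; BeginPlay starts DelayLoop, a self-calling event that waits a second, then passes a DoN gate capped at twenty repeats.
; Each pass prints the count and runs a ForLoop that colors index messages from a literal color array.
; WhileLoop (with a Delay in its body) and ForEach examples exist but are never called.
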(event Custom|Delay%20Loop
  (Development|PrintText (Utilities|Text|FormatText "This has run {count} times" (stale _counter)))
  (Utilities|FlowControl|Delay 1.0)
  (bind _counter (Utilities|FlowControl|DoN 20)
    (:Exit
      (CallFunction|StartforLoop)
      (CallFunction|DelayLoop) ; Restarts the Loop
    )))

(event Custom|Start%20For%20Loop
  (bind _array (Utilities|Array|MakeArray "(R=0.319566,G=0.669901,B=1.000000,A=1.000000)" "(R=0.298824,G=0.215684,B=1.000000,A=1.000000)" "(R=0.627836,G=1.000000,B=0.421495,A=1.000000)" "(R=1.000000,G=0.347200,B=0.558946,A=1.000000)" "(R=1.000000,G=0.701425,B=0.399781,A=1.000000)" "(R=1.000000,G=0.904841,B=0.646376,A=1.000000)"))
  (for _index (range 0 (- (Utilities|Array|Length _array) 1) 2)
    (Development|PrintText (Utilities|Text|FormatText "This is Index #{index}." _index) true true (Utilities|Array|Get(acopy) _array _index))))

(event Custom|Start%20While%20Loop
  (while (> (Variables|Default|GetWhileLoopCounter) 0) ; Sentinal Loop is a While(True) Loop
    (Development|PrintText (Utilities|Text|FormatText "There are {uses} in this loop." (Variables|Default|GetWhileLoopCounter)) true true "(R=1.000000,G=0.000000,B=0.406494,A=1.000000)")
    (Math|Integer|DecrementInt (Variables|Default|GetWhileLoopCounter)
      (:%20%20
        (Utilities|FlowControl|Delay 0.2)
        (Development|PrintText "after delay" true true "(R=1.000000,G=0.764251,B=0.127234,A=1.000000)"))))
  (Variables|Default|SetWhileLoopCounter 10))

(event Custom|Start%20For%20Each%20Loop
  (for (_array_element _array_index) (Utilities|Array|MakeArray "(R=0.319566,G=0.669901,B=1.000000,A=1.000000)" "(R=0.298824,G=0.215684,B=1.000000,A=1.000000)" "(R=0.627836,G=1.000000,B=0.421495,A=1.000000)" "(R=1.000000,G=0.347200,B=0.558946,A=1.000000)" "(R=1.000000,G=0.701425,B=0.399781,A=1.000000)" "(R=1.000000,G=0.904841,B=0.646376,A=1.000000)")
    (Development|PrintText (Utilities|Text|FormatText "This is Index #{index}." _array_index) true true _array_element)))

(event EventBeginPlay
  (Development|PrintString "Loops and Lists BP Exists")
  (CallFunction|DelayLoop))

(event Collision|EventActorBeginOverlap
  (params (OtherActor :type Actor%20Object%20Reference)))

(event EventTick
  (params (DeltaSeconds :type Float%20%28single-precision%29)))

(fn ConstructionScript)