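; Game instance Blueprint that saves the player's state to a named save slot.
; SaveGame loads the existing SG_coding2 object from the slot, or creates one if none exists.
; It then copies the third-person character's stamina, capsule world transform and sprint and shoot flags into that object and writes it back.
; LoadGame is only a stub that prints a start message and restores nothing.
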(event Custom|SaveGame
  (Development|PrintString "Starting Save Game")
  (bind _returnvalue (SaveGame|DoesSaveGameExist (Variables|Default|GetSlot%20Name))) ; have we already saved before?
  (if _returnvalue ; True if we've saved before.
    (bind _returnvalue_2 (SaveGame|LoadGamefromSlot (Variables|Default|GetSlot%20Name))) ; load our previous save file
    (Variables|Default|SetSaver%20Subclass _returnvalue_2)
    (else
      (bind _returnvalue_3 (SaveGame|CreateSaveGameObject "/Game/Blueprints/SG_coding2.SG_coding2_C")) ; create a new save file
      (Variables|Default|SetSaver%20Subclass _returnvalue_3)))
  ;[1 0.8509 0.2252] Save Game Data
  (bind _assg_coding_2 (Utilities|Casting|CastToSG_coding2 (Variables|Default|GetSaver%20Subclass)))
  ;[1 1 1] Player's current data
  (bind _asbp_third_person_character (Utilities|Casting|CastToBP_ThirdPersonCharacter (Game|GetPlayerCharacter 0))) ; get a reference to the player
  (Variables|/Game/Blueprints/SG_coding2.SG_coding2_C|SetPlayerStamina _assg_coding_2 (Variables|/Game/ThirdPerson/Blueprints/BP_ThirdPersonCharacter.BP_ThirdPersonCharacter_C|GetStamina _asbp_third_person_character))
  (Variables|/Game/Blueprints/SG_coding2.SG_coding2_C|SetPlayerTransform _assg_coding_2 (Transformation|GetWorldTransform (Variables|/Script/Engine.Character|GetCapsuleComponent _asbp_third_person_character)))
  (Variables|/Game/Blueprints/SG_coding2.SG_coding2_C|SetPlayerCanSprint _assg_coding_2 (Variables|/Game/ThirdPerson/Blueprints/BP_ThirdPersonCharacter.BP_ThirdPersonCharacter_C|GetCanSprint _asbp_third_person_character))
  (Variables|/Game/Blueprints/SG_coding2.SG_coding2_C|SetPlayerCanShoot _assg_coding_2 (Variables|/Game/ThirdPerson/Blueprints/BP_ThirdPersonCharacter.BP_ThirdPersonCharacter_C|GetCanShoot _asbp_third_person_character))
  (SaveGame|SaveGametoSlot _assg_coding_2 (Variables|Default|GetSlot%20Name))
  (Development|PrintString "game is successfully sved" true true "(R=0.000000,G=0.660000,B=0.000000,A=1.000000)"))

(event Custom|Load%20Game
  (Development|PrintString "Starting Load Game"))